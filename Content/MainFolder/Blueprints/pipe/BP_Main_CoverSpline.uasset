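; Pipe cover spline actor that builds a run of deformed meshes along an editable spline, with no runtime logic.
; The construction script adds one spline mesh per whole MeshLength of spline distance, leaving any remainder uncovered, and applies a shared mesh and material.
; Tangents are clamped to MeshLength so each fixed-length piece bends along the curve.
; An alternative per-spline-point builder without collision remains disconnected.
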(fn `UserConstructionScript`
  (bind _meshlength (`self.MeshLength`))
  (bind _meshlength_2 (`self.MeshLength`))
  ;[1 1 1] 2 way better connection
  (for _index (range (+ (`KismetMathLibrary.FTrunc` (- (/ (`SplineComponent.GetSplineLength` (`self.Spline`)) (`self.MeshLength`)) 1.0)) 1))
    (bind _returnvalue (`AddComponent|NODE_AddSplineMeshComponent-2`))
    (`StaticMeshComponent.SetStaticMesh` _returnvalue (`self.Static Mesh`))
    (bind _returnvalue_2 (* _index _meshlength))
    (bind _returnvalue_3 (* (+ _index 1) _meshlength))
    (`SplineMeshComponent.SetStartAndEnd` _returnvalue (`SplineComponent.GetLocationAtDistanceAlongSpline` (`self.Spline`) _returnvalue_2 "Local") (`KismetMathLibrary.ClampVectorSize` (`SplineComponent.GetTangentAtDistanceAlongSpline` (`self.Spline`) _returnvalue_2 "Local") 0.0 _meshlength_2) (`SplineComponent.GetLocationAtDistanceAlongSpline` (`self.Spline`) _returnvalue_3 "Local") (`KismetMathLibrary.ClampVectorSize` (`SplineComponent.GetTangentAtDistanceAlongSpline` (`self.Spline`) _returnvalue_3 "Local") 0.0 _meshlength_2) true)
    (`PrimitiveComponent.SetMaterial` _returnvalue 0 (`self.Material`))))